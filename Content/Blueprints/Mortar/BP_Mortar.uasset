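; BP_Mortar is a mortar actor built on the tank aiming setup, with a barrel, a dome that serves as turret, and a health bar widget.
; On BeginPlay it initializes its aiming component with the barrel and dome.
; It then casts the health bar widget component's user widget to W_HealthBar_BP and sets itself as that widget's TankRef.
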(event `self.ReceiveBeginPlay`
  (`TankAimingComponent.Initialize` (`self.BP_TankAimingComponent`) (`self.BP_Barrel`) (`self.BP_Dome`))
  (`self.Initialize_HealthBar`))

(fn `Initialize_HealthBar`
  (bind _asw_health_bar_bp (cast `/Game/UI/W_HealthBar_BP` (`WidgetComponent.GetUserWidgetObject` (`self.W_HealthBar`))))
  (set `/Game/UI/W_HealthBar_BP.Tank_Ref` self _asw_health_bar_bp))

(fn `UserConstructionScript`)