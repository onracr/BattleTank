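; BP_Tank is the player-controllable tank pawn, wiring its aiming and movement components to the barrel, turret and tracks on BeginPlay.
; It also hands itself to its health bar widget.
; Input rotates an azimuth gimbal and spring arm for camera aim, zooms the arm and toggles first- and third-person cameras.
; Fire and movement axes are forwarded to the aiming and movement components.
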(event `self.ReceiveBeginPlay`
  (`TankAimingComponent.Initialize` (`self.BP_TankAimingComponent`) (`self.BP_TankBarrel`) (`self.BP_TankTurret`))
  (`TankMovementComponent.Initialize` (`self.BP_TankMovementComponent`) (`self.BP_TankTrack_L`) (`self.BP_TankTrack_R`))
  (bind _asw_health_bar_bp (cast `/Game/UI/W_HealthBar_BP` (`WidgetComponent.GetUserWidgetObject` (`self.W_HealthBar`))))
  (set `/Game/UI/W_HealthBar_BP.Tank_Ref` self _asw_health_bar_bp))

(event `InputAxis|AimAzimuth`
  (params (AxisValue :type "Float (single-precision)"))
  ;[1 1 1] Ballistics Input Binding
  (`SceneComponent.K2_AddLocalRotation` (`self.AzimuthGimbal`) (`KismetMathLibrary.MakeRotator` 0.0 0.0 (* AxisValue (`GameplayStatics.GetWorldDeltaSeconds`) 100.0)) false false))

(event `InputAction|TPS_Camera_Zoom_In`
  (params (Key :type "Key Structure"))
  ;[1 1 1] Camera Zoom
  (:`Pressed`
    (set `SpringArmComponent.TargetArmLength` (- (`SpringArmComponent.TargetArmLength` (`self.SpringArm`)) 25.0) (`self.SpringArm`))))

(event `InputAxis|AimElevation`
  (params (AxisValue :type "Float (single-precision)"))
  ;[1 1 1] Ballistics Input Binding
  (`SceneComponent.K2_AddLocalRotation` (`self.SpringArm`) (`KismetMathLibrary.MakeRotator` 0.0 (* AxisValue (`GameplayStatics.GetWorldDeltaSeconds`) 100.0)) false false))

(event `InputAction|TPS_Camera_Zoom_Out`
  (params (Key :type "Key Structure"))
  ;[1 1 1] Camera Zoom
  (:`Pressed`
    (set `SpringArmComponent.TargetArmLength` (+ (`SpringArmComponent.TargetArmLength` (`self.SpringArm`)) 25.0) (`self.SpringArm`))))

(event `InputAction|Fire`
  (params (Key :type "Key Structure"))
  ;[1 1 1] Ballistics Input Binding
  (:`Pressed`
    (`TankAimingComponent.Fire` (`self.BP_TankAimingComponent`))))

(event `InputAction|Switch_Cam`
  (params (Key :type "Key Structure"))
  ;[1 1 1] FPS-TPS Toggle
  (:`Pressed`
    (`ActorComponent.ToggleActive` (`self.FPS_Camera`))
    (`ActorComponent.ToggleActive` (`self.TPS_Camera`))))

(event `InputAxis|MoveForward`
  (params (AxisValue :type "Float (single-precision)"))
  ;[1 1 1] Movement Input Binding
  (`TankMovementComponent.IntendMoveForward` (`self.BP_TankMovementComponent`) AxisValue))

(event `InputAxis|TurnRight`
  (params (AxisValue :type "Float (single-precision)"))
  ;[1 1 1] Movement Input Binding
  (`TankMovementComponent.IntendTurnRight` (`self.BP_TankMovementComponent`) AxisValue))

(fn `UserConstructionScript`)